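; BP_TestTrigger is a developer test trigger that plays a level sequence for all players when a player character enters its Box.
; On overlap it checks for a USACharacterPlayer, a valid game mode and an assigned InLevelSequence, then asks the USAGameModeBase to play that sequence.
; The IsActived flag is set on first activation, so the trigger fires only once.
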(event OnComponentBeginOverlap(Box)
  (params (OverlappedComponent :type Primitive%20Component%20Object%20Reference) (OtherActor :type Actor%20Object%20Reference) (OtherComp :type Primitive%20Component%20Object%20Reference) (OtherBodyIndex :type Integer) (bFromSweep :type Boolean) (SweepResult :type Hit%20Result%20Structure%20%28by%20ref%29))
  (bind _returnvalue (Game|GetGameMode))
  (Utilities|Casting|CastToUSACharacterPlayer OtherActor)
  (Utilities|IsValid _returnvalue
    (:Is%20Valid
      (Utilities|IsValid (Variables|Default|GetInLevelSequence)
        (:Is%20Valid
          (if (not (Variables|Default|GetbIsActived))
            (Variables|Default|SetbIsActived true)
            (bind _asusagame_mode_base (Utilities|Casting|CastToUSAGameModeBase _returnvalue))
            (Class|USAGameModeBase|PlayLevelSequencetoAllPlayer _asusagame_mode_base (Variables|Default|GetInLevelSequence))))))))

(event EventBeginPlay)

(event Collision|EventActorBeginOverlap
  (params (OtherActor :type Actor%20Object%20Reference)))

(event EventTick
  (params (DeltaSeconds :type Float%20%28single-precision%29)))

(fn ConstructionScript)