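; BP_TestTriggerSingle is a test trigger volume that starts a level sequence once when a player character enters its box.
; On overlap it checks that the character has a valid local player controller and that a sequence is assigned.
; It then sets a one-shot flag and asks the USA game state to play the sequence through PlayLevelSequenceSingle.
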(event OnComponentBeginOverlap(Box)
  (params (OverlappedComponent :type Primitive%20Component%20Object%20Reference) (OtherActor :type Actor%20Object%20Reference) (OtherComp :type Primitive%20Component%20Object%20Reference) (OtherBodyIndex :type Integer) (bFromSweep :type Boolean) (SweepResult :type Hit%20Result%20Structure%20%28by%20ref%29))
  (bind _asusacharacter_player (Utilities|Casting|CastToUSACharacterPlayer OtherActor))
  (Utilities|IsValid (Variables|/Script/ProjectUSA.USACharacterPlayer|GetLocalUSAPlayerController _asusacharacter_player)
    (:Is%20Valid
      (bind _asusagame_state_base (Utilities|Casting|CastToUSAGameStateBase (Game|GetGameState)))
      (Utilities|IsValid (Variables|Default|GetInLevelSequence)
        (:Is%20Valid
          (if (not (Variables|Default|GetbIsActived))
            (Variables|Default|SetbIsActived true)
            (Class|USAGameStateBase|PlayLevelSequenceSingle _asusagame_state_base (Variables|Default|GetInLevelSequence))))))))

(event EventBeginPlay)

(event Collision|EventActorBeginOverlap
  (params (OtherActor :type Actor%20Object%20Reference)))

(event EventTick
  (params (DeltaSeconds :type Float%20%28single-precision%29)))

(fn ConstructionScript)