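; Game instance Blueprint that provides events for hosting and joining multiplayer games over LAN or by IP address.
; Hosting opens the given level as a listen server, first creating a four-slot LAN session when the LAN flag is set.
; LAN joining searches for sessions and joins the first result, while IP joining passes the address to Open Level.
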(event EventJoinSessionbyLAN
  (params (InPlayerController :type Player%20Controller%20Object%20Reference))
  ;[1 1 1] Comment
  (bind _results (|FindSessions InPlayerController 100 true)
    (:OnSuccess
      (|JoinSession InPlayerController (Utilities|Array|Get(acopy) _results)))))

(event EventHostSession
  (params (InPlayerController :type Player%20Controller%20Object%20Reference) (InLevelName :type Name :default "None") (InLAN :type Boolean))
  ;[1 1 1] Comment
  (if InLAN
    (|Session InPlayerController 4 true
      (:OnSuccess
        _)))
  (Game|OpenLevel(byName) InLevelName true "?listen"))

(event EventJoinSessionbyIPAddress
  (params (InPlayerController :type Player%20Controller%20Object%20Reference) (InIP :type Text%20%28by%20ref%29))
  ;[1 1 1] Comment
  (Game|OpenLevel(byName) (Utilities|String|StringToName (Utilities|String|ToString(Text) InIP))))