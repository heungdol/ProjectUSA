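; BP_RingPath is a ring actor that reacts when a local player air-dashes through it.
; On begin play it binds its RingHolder component to a jelly effect component.
; When the box trigger overlaps a locally controlled player character whose ability system has the AirDash action tag, it plays the configured jelly wobble effect.
; The reaction is purely local feedback; no other gameplay effect is applied here.
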(event OnComponentBeginOverlap(Box)
  (params (OverlappedComponent :type Primitive%20Component%20Object%20Reference) (OtherActor :type Actor%20Object%20Reference) (OtherComp :type Primitive%20Component%20Object%20Reference) (OtherBodyIndex :type Integer) (bFromSweep :type Boolean) (SweepResult :type Hit%20Result%20Structure%20%28by%20ref%29))
  (bind _asusacharacter_player (Utilities|Casting|CastToUSACharacterPlayer OtherActor))
  (Utilities|IsValid (Pawn|GetController _asusacharacter_player)
    (:Is%20Valid
      (if (and (Pawn|IsLocalController (Pawn|GetController _asusacharacter_player)) (GameplayTags|HasMatchingGameplayTag (Ability|GetAbilitySystemComponent _asusacharacter_player) "(TagName=\"Character.Action.AirDash\")"))
        (Class|USAJellyEffectComponent|PlayJellyEffect (Variables|Default|GetUSAJellyEffect) (Variables|Default|GetJellyEffectData_Path))))))

(event EventBeginPlay
  (Class|USAJellyEffectComponent|SetJellySceneComponent (Variables|Default|GetUSAJellyEffect) 0 (Variables|Default|GetRingHolder)))

(event Collision|EventActorBeginOverlap
  (params (OtherActor :type Actor%20Object%20Reference)))

(event EventTick
  (params (DeltaSeconds :type Float%20%28single-precision%29)))

(fn ConstructionScript)