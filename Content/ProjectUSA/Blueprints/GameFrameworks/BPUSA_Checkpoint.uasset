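; BPUSA_Checkpoint is a checkpoint actor whose mesh and effect reflect whether it is active.
; It hides its static mesh on BeginPlay, then OnCheckpointUpdated toggles the mesh visibility to match the active state.
; On activation it spawns the NS_USA_Checkpoint effect attached to the mesh, using IsPlayedVFX to avoid replays until it is deactivated again.
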(event EventBeginPlay
  (Rendering|SetVisibility (Variables|Default|GetStaticMesh) false true))

(event Collision|EventActorBeginOverlap
  (params (OtherActor :type Actor%20Object%20Reference)))

(event EventTick
  (params (DeltaSeconds :type Float%20%28single-precision%29)))

(event EventOnCheckpointUpdated
  (params (bIsActive :type Boolean))
  (Utilities|FlowControl|Sequence
    (:then_0
      (Rendering|SetVisibility (Variables|Default|GetStaticMesh) bIsActive true))
    (:then_1
      (if bIsActive
        (if (not (Variables|Default|GetIsPlayedVFX))
          (Niagara|SpawnSystemAttached "/Game/ProjectUSA/VisualEffects/NiagaraEffects/NS_USA_Checkpoint.NS_USA_Checkpoint" (Variables|Default|GetStaticMesh) "None" "0, 0, 0" "0, 0, 0" "KeepRelativeOffset" true)
          (Variables|Default|SetIsPlayedVFX true))
        (else
          (Variables|Default|SetIsPlayedVFX false))))))

(fn ConstructionScript)