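; Base Blueprint for AI enemy characters, built on a USACharacter parent, that links character events to animation, UI and AI.
; Crouch and death events set flags on the ABP_Manny anim Blueprint.
; BeginPlay labels the nickname widget "AI", and health ratio changes drive the health bar widget.
; On possession it passes its StartBT to the BPUSA_AIController, so each enemy can supply its own behavior tree.
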(event EventBeginPlay
  (Utilities|FlowControl|Sequence
    (:then_0
      ;[1 1 1] USACharacter - Adding Charater NickName (AI)
      (bind _aswbp_nickname_utility (Utilities|Casting|CastToWBP_Nickname_Utility (UserInterface|GetWidget (Variables|Default|GetNicknameWidgetComponent))))
      (Variables|/Script/UMG.TextBlock|SetText (Variables|/Game/ProjectUSA/UI/WBP_Nickname_Utility.WBP_Nickname_Utility_C|GetNickNameContent _aswbp_nickname_utility) "AI"))))

(event EventOnCurrentHealthRatioChanged
  (params (InValue :type Float%20%28single-precision%29))
  ;[1 1 1] USACharacter - Change HealthBar using Current / Max Health
  (bind _aswbp_character_health_bar (Utilities|Casting|CastToWBP_CharacterHealthBar (UserInterface|GetWidget (Variables|Default|GetHealthBarWidgetComponent))))
  (Progress|SetPercent (Variables|/Game/ProjectUSA/UI/WBP_CharacterHealthBar.WBP_CharacterHealthBar_C|GetHealthBar _aswbp_character_health_bar) InValue))

(event EventOnUSADeath
  ;[1 1 1] USACharacter - Death
  (bind _asabp_manny (Utilities|Casting|CastToABP_Manny (Components|SkeletalMesh|GetAnimInstance (Variables|Character|GetMesh))))
  (Variables|/Game/Characters/Mannequins/Animations/ABP_Manny.ABP_Manny_C|SetIsDead _asabp_manny true))

(event EventOnStartCrouch
  (params (HalfHeightAdjust :type Float%20%28single-precision%29) (ScaledHalfHeightAdjust :type Float%20%28single-precision%29))
  ;[1 1 1] USACharacter - Sending Crouch Animation Info to Anim Blueprint
  (bind _asabp_manny (Utilities|Casting|CastToABP_Manny (Components|SkeletalMesh|GetAnimInstance (Variables|Character|GetMesh))))
  (Variables|/Game/Characters/Mannequins/Animations/ABP_Manny.ABP_Manny_C|SetIsCrouching _asabp_manny true))

(event EventOnEndCrouch
  (params (HalfHeightAdjust :type Float%20%28single-precision%29) (ScaledHalfHeightAdjust :type Float%20%28single-precision%29))
  ;[1 1 1] USACharacter - Sending Crouch Animation Info to Anim Blueprint
  (bind _asabp_manny (Utilities|Casting|CastToABP_Manny (Components|SkeletalMesh|GetAnimInstance (Variables|Character|GetMesh))))
  (Variables|/Game/Characters/Mannequins/Animations/ABP_Manny.ABP_Manny_C|SetIsCrouching _asabp_manny false))

(event Collision|EventActorBeginOverlap
  (params (OtherActor :type Actor%20Object%20Reference)))

(event EventTick
  (params (DeltaSeconds :type Float%20%28single-precision%29)))

(event EventPossessed
  (params (NewController :type Controller%20Object%20Reference))
  ;[1 1 1] USACharacter - Setting Start BT for AI
  (bind _asbpusa_aicontroller (Utilities|Casting|CastToBPUSA_AIController NewController))
  (Variables|/Game/ProjectUSA/AI/BPUSA_AIController.BPUSA_AIController_C|SetStartBT _asbpusa_aicontroller (Variables|Default|GetStartBT)))

(fn ConstructionScript)