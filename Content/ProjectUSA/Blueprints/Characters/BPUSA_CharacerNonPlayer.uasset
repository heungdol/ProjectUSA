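; Non-player character Blueprint for ProjectUSA that passes its crouch state to the animation Blueprint.
; The crouch start and end events cast the mesh's anim instance to ABP_Manny and set its IsCrouching flag.
; BeginPlay leads to an empty sequence and Tick does nothing.
; Disconnected test logic for spawning a first weapon and printing movement input never runs.
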(event EventBeginPlay
  (Utilities|FlowControl|Sequence))

(event Collision|EventActorBeginOverlap
  (params (OtherActor :type Actor%20Object%20Reference)))

(event EventTick
  (params (DeltaSeconds :type Float%20%28single-precision%29)))

(event EventOnStartCrouch
  (params (HalfHeightAdjust :type Float%20%28single-precision%29) (ScaledHalfHeightAdjust :type Float%20%28single-precision%29))
  ;[1 1 1] USACharacter - Sending Crouch Animation Info to Anim Blueprint
  (bind _asabp_manny (Utilities|Casting|CastToABP_Manny (Components|SkeletalMesh|GetAnimInstance (Variables|Character|GetMesh))))
  (Variables|/Game/Characters/Mannequins/Animations/ABP_Manny.ABP_Manny_C|SetIsCrouching _asabp_manny true))

(event EventOnEndCrouch
  (params (HalfHeightAdjust :type Float%20%28single-precision%29) (ScaledHalfHeightAdjust :type Float%20%28single-precision%29))
  ;[1 1 1] USACharacter - Sending Crouch Animation Info to Anim Blueprint
  (bind _asabp_manny (Utilities|Casting|CastToABP_Manny (Components|SkeletalMesh|GetAnimInstance (Variables|Character|GetMesh))))
  (Variables|/Game/Characters/Mannequins/Animations/ABP_Manny.ABP_Manny_C|SetIsCrouching _asabp_manny false))

(fn ConstructionScript)