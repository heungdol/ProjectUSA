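; Weapon spawner actor that spawns an instance of its configured weapon class at its own transform on BeginPlay, on the server only.
; The construction script reads that class's defaults and applies its skeletal and static meshes to the spawner's own mesh components, so the spawner displays the selected weapon's meshes.
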(event EventBeginPlay
  (if (Networking|IsServer)
    (Game|SpawnActorfromClass (Variables|Default|GetSpawnWeaponBaseClass) (Transformation|GetActorTransform) "Undefined" "MultiplyWithRoot" 0 0)))

(event Collision|EventActorBeginOverlap
  (params (OtherActor :type Actor%20Object%20Reference)))

(event EventTick
  (params (DeltaSeconds :type Float%20%28single-precision%29)))

(fn ConstructionScript
  (bind _spawnweaponbaseclass (Variables|Default|GetSpawnWeaponBaseClass))
  (bind (_weaponskeletalmeshmeshref _weaponstaticmeshref) (Utilities|GetClassDefaults _spawnweaponbaseclass))
  (Utilities|FlowControl|Sequence
    (:then_0
      (Components|SkeletalMesh|SetSkeletalMeshAsset (Variables|Default|GetSkeletalMesh) _weaponskeletalmeshmeshref))
    (:then_1
      (Components|StaticMesh|SetStaticMesh (Variables|Default|GetStaticMesh) _weaponstaticmeshref))))