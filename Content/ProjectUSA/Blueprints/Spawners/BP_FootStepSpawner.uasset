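; BP_FootStepSpawner is a trigger actor that spawns an AI pawn, labeled as an enemy, when a player character steps into its box.
; The box overlap runs only on server or standalone and counts only the player's parentless component, then spawns the configured class and behavior tree at SpawnPoint's transform.
; Each qualifying overlap spawns again, and BeginPlay sets the SpawnText label from SpawnTextContent.
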(event OnComponentBeginOverlap(Box)
  (params (OverlappedComponent :type Primitive%20Component%20Object%20Reference) (OtherActor :type Actor%20Object%20Reference) (OtherComp :type Primitive%20Component%20Object%20Reference) (OtherBodyIndex :type Integer) (bFromSweep :type Boolean) (SweepResult :type Hit%20Result%20Structure%20%28by%20ref%29))
  (bind _spawnpoint (Variables|Default|GetSpawnPoint))
  ;[1 1 1] USA - FootStep Spawning Enemy
  (Utilities|Casting|CastToBPUSA_CharacerPlayer OtherActor)
  (if (and (or (Networking|IsServer) (Class|KismetSystemLibrary|IsStandalone)) (== (Utilities|Array|Length (Class|SceneComponent|GetParentComponents OtherComp)) 0))
    (AI|SpawnAIFromClass (Variables|Default|GetSpawnAIClass) (Variables|Default|GetSpawnBT) (Transformation|GetWorldLocation _spawnpoint) (Transformation|GetWorldRotation _spawnpoint) false 0)))

(event EventBeginPlay
  (Rendering|Components|TextRender|SetText (Variables|Default|GetSpawnText) (Variables|Default|GetSpawnTextContent)))

(event Collision|EventActorBeginOverlap
  (params (OtherActor :type Actor%20Object%20Reference)))

(event EventTick
  (params (DeltaSeconds :type Float%20%28single-precision%29)))

(fn ConstructionScript)