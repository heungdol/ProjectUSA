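; Player character Blueprint for ProjectUSA that relays crouch state to the mesh's animation Blueprint.
; On crouch start and end, it casts the mesh's anim instance to ABP_Manny and sets IsCrouching.
; BeginPlay, Tick, overlap and the construction script are empty.
; Unconnected nodes for slide montage playback and a mesh location offset remain in the graph but never run.
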(event EventBeginPlay)

(event Collision|EventActorBeginOverlap
  (params (OtherActor :type Actor%20Object%20Reference)))

(event EventTick
  (params (DeltaSeconds :type Float%20%28single-precision%29)))

(event EventOnStartCrouch
  (params (HalfHeightAdjust :type Float%20%28single-precision%29) (ScaledHalfHeightAdjust :type Float%20%28single-precision%29))
  (bind _asabp_manny (Utilities|Casting|CastToABP_Manny (Components|SkeletalMesh|GetAnimInstance (Variables|Character|GetMesh))))
  (Variables|/Game/Characters/Mannequins/Animations/ABP_Manny.ABP_Manny_C|SetIsCrouching _asabp_manny true))

(event EventOnEndCrouch
  (params (HalfHeightAdjust :type Float%20%28single-precision%29) (ScaledHalfHeightAdjust :type Float%20%28single-precision%29))
  (bind _asabp_manny (Utilities|Casting|CastToABP_Manny (Components|SkeletalMesh|GetAnimInstance (Variables|Character|GetMesh))))
  (Variables|/Game/Characters/Mannequins/Animations/ABP_Manny.ABP_Manny_C|SetIsCrouching _asabp_manny false))

(event Input|KeyboardEvents|Q
  (params (Key :type Key%20Structure :default "None")))

(fn ConstructionScript)