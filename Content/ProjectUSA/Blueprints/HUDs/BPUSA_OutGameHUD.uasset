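; Out-game HUD Blueprint that manages a full-screen panel widget for screen transitions.
; On BeginPlay it creates WBP_Screen_Panel, adds it to the viewport and plays its black animation, then its show animation after a short delay.
; Custom events forward show and hide requests to the panel when it is valid.
; The matching black and white events are empty stubs.
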(event EventBeginPlay
  ;[1 1 1] Comment
  (bind _returnvalue (UserInterface|CreateWidget "/Game/ProjectUSA/UI/Common/WBP_Screen_Panel.WBP_Screen_Panel_C"))
  (bind _output_get (Variables|Default|SetScreen_Panel _returnvalue))
  (UserInterface|Viewport|AddtoViewport _output_get 10)
  (Default|PlayAnimationPanelBlack _output_get)
  (Utilities|FlowControl|Delay 0.5)
  (Default|PlayAnimationPanelShow _output_get))

(event Collision|EventActorBeginOverlap
  (params (OtherActor :type Actor%20Object%20Reference)))

(event EventPlayUserWidgetAnimationPanelHide
  (bind _screen_panel (Variables|Default|GetScreen_Panel))
  ;[1 1 1] Comment
  (Utilities|IsValid _screen_panel
    (:Is%20Valid
      (Default|PlayAnimationPanelHide _screen_panel))))

(event EventPlayUserWidgetAnimationPanelBlack
  ;[1 1 1] Comment
)

(event EventPlayUserWidgetAnimationPanelWhite
  ;[1 1 1] Comment
)

(event EventTick
  (params (DeltaSeconds :type Float%20%28single-precision%29)))

(event EventPlayUserWidgetAnimationPanelShow
  (bind _screen_panel (Variables|Default|GetScreen_Panel))
  ;[1 1 1] Comment
  (Utilities|IsValid _screen_panel
    (:Is%20Valid
      (Default|PlayAnimationPanelShow _screen_panel))))

(fn ConstructionScript)