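; In-game HUD that creates and drives the screen widgets for player HUD, how-to-play help, transition panel, boss HP bar and map name.
; BeginPlay adds them to the viewport in layers and plays a delayed black-to-show panel transition.
; Events push health, boss name, weapon and item data into the widgets and toggle their visibility.
; Holding Tab or GamepadSpecialLeft fades in the help screen; the PanelBlack and PanelWhite events are empty.
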(event EventBeginPlay
  ;[1 1 1] Comment
  (Utilities|FlowControl|Sequence
    (:then_0
      (bind _returnvalue (UserInterface|CreateWidget "/Game/ProjectUSA/UI/WBP_Screen_CharacterHUD.WBP_Screen_CharacterHUD_C"))
      (bind _output_get (Variables|Default|SetScreen_PlayerHUD _returnvalue))
      (UserInterface|Viewport|AddtoViewport _output_get 0))
    (:then_1
      (bind _returnvalue_2 (UserInterface|CreateWidget "/Game/ProjectUSA/UI/WBP_Screen_HowToPlay.WBP_Screen_HowToPlay_C"))
      (bind _output_get_2 (Variables|Default|SetScreen_HowToPlay _returnvalue_2))
      (UserInterface|Viewport|AddtoViewport _output_get_2 5))
    (:then_2
      (bind _returnvalue_3 (UserInterface|CreateWidget "/Game/ProjectUSA/UI/WBP_Screen_Panel.WBP_Screen_Panel_C"))
      (bind _output_get_3 (Variables|Default|SetScreen_Panel _returnvalue_3))
      (UserInterface|Viewport|AddtoViewport _output_get_3 10)
      (Default|PlayAnimationPanelBlack _output_get_3)
      (Utilities|FlowControl|Delay 0.5)
      (Default|PlayAnimationPanelShow _output_get_3))
    (:then_3
      (bind _returnvalue_4 (UserInterface|CreateWidget "/Game/ProjectUSA/UI/WBP_Screen_BossHPBar.WBP_Screen_BossHPBar_C"))
      (bind _output_get_4 (Variables|Default|SetScreen_BossPanel _returnvalue_4))
      (UserInterface|Viewport|AddtoViewport _output_get_4 0)
      (Default|PlayAnimationHideBossHpBar _output_get_4))
    (:then_4
      (bind _returnvalue_5 (UserInterface|CreateWidget "/Game/ProjectUSA/UI/WBP_Screen_MapName.WBP_Screen_MapName_C"))
      (bind _output_get_5 (Variables|Default|SetScreen_MapName _returnvalue_5))
      (UserInterface|Viewport|AddtoViewport _output_get_5 0))))

(event Collision|EventActorBeginOverlap
  (params (OtherActor :type Actor%20Object%20Reference)))

(event EventPlayUserWidgetAnimationPanelHide
  (bind _screen_panel (Variables|Default|GetScreen_Panel))
  ;[1 1 1] Comment
  (Utilities|IsValid _screen_panel
    (:Is%20Valid
      (Default|PlayAnimationPanelHide _screen_panel))))

(event EventShowHideUserWidgetPlayerHUD
  (params (bIsShowing :type Boolean))
  (bind _screen_mapname (Variables|Default|GetScreen_MapName))
  (bind _screen_bosspanel (Variables|Default|GetScreen_BossPanel))
  (bind _screen_playerhud (Variables|Default|GetScreen_PlayerHUD))
  (bind _screen_howtoplay (Variables|Default|GetScreen_HowToPlay))
  ;[1 1 1] Comment
  (if bIsShowing
    (UserInterface|Viewport|AddtoViewport _screen_playerhud 0)
    (UserInterface|Viewport|AddtoViewport _screen_howtoplay 5)
    (UserInterface|Viewport|AddtoViewport _screen_bosspanel 0)
    (UserInterface|Viewport|AddtoViewport _screen_mapname 0)
    (else
      (Widget|RemovefromParent _screen_playerhud)
      (Widget|RemovefromParent _screen_howtoplay)
      (Widget|RemovefromParent _screen_bosspanel)
      (Widget|RemovefromParent _screen_mapname))))

(event EventPlayUserWidgetAnimationPanelBlack
  ;[1 1 1] Comment
)

(event EventPlayUserWidgetAnimationPanelWhite
  ;[1 1 1] Comment
)

(event EventShowHideUserWidgetBossHPBar
  (params (bIsShowing :type Boolean))
  ;[1 1 1] Comment
  (Utilities|IsValid (Variables|Default|GetScreen_BossPanel)
    (:Is%20Valid
      (if bIsShowing
        (Default|PlayAnimationShowBossHPBar (Variables|Default|GetScreen_BossPanel))
        (else
          (Default|PlayAnimationHideBossHpBar (Variables|Default|GetScreen_BossPanel)))))))

(event EventUpdateBossHealthRatio
  (params (InRatio :type Float%20%28single-precision%29))
  ;[1 1 1] Comment
  (Progress|SetPercent (Variables|/Game/ProjectUSA/UI/WBP_Screen_BossHPBar.WBP_Screen_BossHPBar_C|GetBossHPBar (Variables|Default|GetScreen_BossPanel)) InRatio))

(event EventTick
  (params (DeltaSeconds :type Float%20%28single-precision%29)))

(event EventUpdateBossName
  (params (InName :type Name :default "None"))
  ;[1 1 1] Comment
  (Variables|/Script/UMG.TextBlock|SetText (Variables|/Game/ProjectUSA/UI/WBP_Screen_BossHPBar.WBP_Screen_BossHPBar_C|GetBossName (Variables|Default|GetScreen_BossPanel)) (Utilities|Text|ToText(Name) InName)))

(event EventUpdatePlayerWeapon
  (params (InType :type EUSAWeaponType%20Enum :default "None") (InWeapon :type USA%20Weapon%20Base%20Object%20Reference))
  (bind _screen_playerhud (Variables|Default|GetScreen_PlayerHUD))
  ;[1 1 1] Comment
  (Utilities|IsValid (Variables|Default|GetScreen_PlayerHUD)
    (:Is%20Valid
      (Utilities|IsValid InWeapon
        (:Is%20Valid
          (Variables|Default|SetScreen_WeaponTextureTemp (Class|USAWeaponBase|GetWeaponTexture InWeapon)))
        (:Is%20Not%20Valid
          (Variables|Default|SetScreen_WeaponTextureTemp "/Game/ProjectUSA/Textures/T2D_None.T2D_None")))
      (switch Utilities|FlowControl|Switch|SwitchonEUSAWeaponType InType
        (:First
          (Appearance|SetBrushfromTexture (Variables|/Game/ProjectUSA/UI/WBP_Screen_CharacterHUD.WBP_Screen_CharacterHUD_C|GetFirstWeaponImage _screen_playerhud) (Variables|Default|GetScreen_WeaponTextureTemp) false))
        (:Second
          (Appearance|SetBrushfromTexture (Variables|/Game/ProjectUSA/UI/WBP_Screen_CharacterHUD.WBP_Screen_CharacterHUD_C|GetSecondWeaponImage _screen_playerhud) (Variables|Default|GetScreen_WeaponTextureTemp) false)))
      (Variables|Default|SetScreen_WeaponTextureTemp 0))))

(event EventPlayUserWidgetAnimationPanelShow
  (bind _screen_panel (Variables|Default|GetScreen_Panel))
  ;[1 1 1] Comment
  (Utilities|IsValid _screen_panel
    (:Is%20Valid
      (Default|PlayAnimationPanelShow _screen_panel))))

(event EventUpdatePlayerHPBar
  (params (InRatio :type Float%20%28single-precision%29))
  ;[1 1 1] Comment
  (Utilities|IsValid (Variables|Default|GetScreen_PlayerHUD)
    (:Is%20Valid
      (Progress|SetPercent (Variables|/Game/ProjectUSA/UI/WBP_Screen_CharacterHUD.WBP_Screen_CharacterHUD_C|GetHPBar (Variables|Default|GetScreen_PlayerHUD)) InRatio))))

(event EventChangePlayerItem
  (params (InItemClass :type USA%20Item%20Base%20Class%20Reference))
  (bind _screen_playerhud (Variables|Default|GetScreen_PlayerHUD))
  (bind _itemimage (Variables|/Game/ProjectUSA/UI/WBP_Screen_CharacterHUD.WBP_Screen_CharacterHUD_C|GetItemImage _screen_playerhud))
  ;[1 1 1] Comment
  (Utilities|IsValid _screen_playerhud
    (:Is%20Valid
      (if (Utilities|IsValidClass InItemClass)
        (Appearance|SetBrushfromTexture _itemimage (.ItemTexture (Utilities|GetClassDefaults InItemClass)) false)
        (else
          (Appearance|SetBrushfromTexture _itemimage "/Game/ProjectUSA/Textures/T2D_None.T2D_None" false))))))

(event EventChangePlayerItemCount
  (params (InItemCount :type Integer))
  (bind _screen_playerhud (Variables|Default|GetScreen_PlayerHUD))
  ;[1 1 1] Comment
  (Utilities|IsValid _screen_playerhud
    (:Is%20Valid
      (Rendering|Components|TextRender|SetText (Variables|/Game/ProjectUSA/UI/WBP_Screen_CharacterHUD.WBP_Screen_CharacterHUD_C|GetItemCount _screen_playerhud) (Utilities|Text|ToText(Integer) InItemCount)))))

(event Input|KeyboardEvents|Tab
  (params (Key :type Key%20Structure :default "None"))
  ;[1 1 1] USA - Show How to Play?
  (:Pressed
    (Utilities|IsValid (Variables|Default|GetScreen_HowToPlay)
      (:Is%20Valid
        (Default|PlayAnimationFadein (Variables|Default|GetScreen_HowToPlay)))))
  (:Released
    (Utilities|IsValid (Variables|Default|GetScreen_HowToPlay)
      (:Is%20Valid
        (Default|PlayAnimationFadeOut (Variables|Default|GetScreen_HowToPlay))))))

(event Input|GamepadEvents|GamepadSpecialLeft
  (params (Key :type Key%20Structure :default "None"))
  ;[1 1 1] USA - Show How to Play?
  (:Pressed
    (Utilities|IsValid (Variables|Default|GetScreen_HowToPlay)
      (:Is%20Valid
        (Default|PlayAnimationFadein (Variables|Default|GetScreen_HowToPlay)))))
  (:Released
    (Utilities|IsValid (Variables|Default|GetScreen_HowToPlay)
      (:Is%20Valid
        (Default|PlayAnimationFadeOut (Variables|Default|GetScreen_HowToPlay))))))

(fn ConstructionScript)