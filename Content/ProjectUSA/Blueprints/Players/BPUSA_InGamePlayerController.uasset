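; In-game player controller that sets up the local player's screen UI and tracks gamepad use.
; On BeginPlay it layers the character HUD, How to Play and screen panel widgets by Z-order, with the panel going black before revealing after a short delay.
; Holding Tab fades How to Play in, and releasing fades it out.
; Any key press reports whether it came from a gamepad to USAPlayerState.
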(event EventBeginPlay
  ;[1 1 1] USA - Set Screen UI (HUD)
  (if (Pawn|IsLocalPlayerController)
    (Utilities|FlowControl|Sequence
      (:then_0
        (bind _returnvalue (UserInterface|CreateWidget "/Game/ProjectUSA/UI/WBP_CharacterHUD.WBP_CharacterHUD_C"))
        (Utilities|IsValid _returnvalue
          (:Is%20Valid
            (bind _output_get (Variables|Default|SetPlayerHUDUserWidget _returnvalue))
            (UserInterface|Viewport|AddtoViewport _output_get 0))))
      (:then_1
        (bind _returnvalue_2 (UserInterface|CreateWidget "/Game/ProjectUSA/UI/WBP_HowToPlay.WBP_HowToPlay_C"))
        (bind _output_get_2 (Variables|Default|SetHowToPlay _returnvalue_2))
        (UserInterface|Viewport|AddtoViewport _output_get_2 5))
      (:then_2
        (bind _returnvalue_3 (UserInterface|CreateWidget "/Game/ProjectUSA/UI/WBP_ScreenPanel.WBP_ScreenPanel_C"))
        (UserInterface|Viewport|AddtoViewport _returnvalue_3 10)
        (bind _output_get_3 (Variables|Default|SetScreenPanel _returnvalue_3))
        (Default|PlayAnimationPanelBlack _output_get_3)
        (Utilities|FlowControl|Delay 0.5)
        (Default|PlayAnimationPanelShow _output_get_3)))))

(event EventTick
  (params (DeltaSeconds :type Float%20%28single-precision%29)))

(event EventPossess
  (params (PossessedPawn :type Pawn%20Object%20Reference))
  ;[1 1 1] Comment
)

(event Input|KeyboardEvents|AnyKey
  (params (Key :type Key%20Structure :default "None"))
  ;[1 1 1] USA - Send Current Gamepad State to USAPlayerState
  (:Pressed
    (bind _asusaplayer_state (Utilities|Casting|CastToUSAPlayerState (Variables|Default|GetPlayerState)))
    (Class|USAPlayerState|SetIsUsingGamepad _asusaplayer_state (Class|KismetInputLibrary|KeyIsGamepadKey Key))))

(event Input|KeyboardEvents|Tab
  (params (Key :type Key%20Structure :default "None"))
  ;[1 1 1] USA - Show How to Play?
  (:Pressed
    (Utilities|IsValid (Variables|Default|GetHowToPlay)
      (:Is%20Valid
        (Default|PlayAnimationFadein (Variables|Default|GetHowToPlay)))))
  (:Released
    (Utilities|IsValid (Variables|Default|GetHowToPlay)
      (:Is%20Valid
        (Default|PlayAnimationFadeOut (Variables|Default|GetHowToPlay))))))

(fn ConstructionScript)