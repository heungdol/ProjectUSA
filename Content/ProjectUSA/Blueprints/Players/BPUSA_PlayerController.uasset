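; Player controller for ProjectUSA that creates the on-screen character HUD and tracks whether the player is using a gamepad.
; On BeginPlay, the local controller creates the WPB_CharacterHUD widget, adds it to the viewport and stores a reference.
; Any key press checks whether the key is a gamepad key and passes the result to USAPlayerState.
; An unconnected branch that would show a multiplayer listen menu never runs.
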(event EventBeginPlay
  ;[1 1 1] USA - Set Screen UI (HUD)
  (if (Pawn|IsLocalPlayerController)
    (Utilities|FlowControl|Sequence
      (:then_0
        (bind _returnvalue (UserInterface|CreateWidget "/Game/ProjectUSA/UI/WPB_CharacterHUD.WPB_CharacterHUD_C"))
        (Utilities|IsValid _returnvalue
          (:Is%20Valid
            (UserInterface|Viewport|AddtoViewport _returnvalue 0)
            (Variables|Default|SetCharacterHUD _returnvalue)))))))

(event EventTick
  (params (DeltaSeconds :type Float%20%28single-precision%29)))

(event Input|KeyboardEvents|AnyKey
  (params (Key :type Key%20Structure :default "None"))
  (:Pressed
    ;[1 1 1] USA - Send Current Gamepad State to USAPlayerState
    (bind _asusaplayer_state (Utilities|Casting|CastToUSAPlayerState (Variables|Default|GetPlayerState)))
    (Class|USAPlayerState|SetIsUsingGamepad _asusaplayer_state (Class|KismetInputLibrary|KeyIsGamepadKey Key))))

(fn ConstructionScript)