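; In-game GameState that drives the local player's boss health UI and cutscene playback.
; Boss bar visibility, health ratio and name events forward to the local HUD.
; Sequence events disable player input, hide the character HUD behind animated panel transitions, play the Level Sequence, then restore both after a duration-based delay.
; Multi sequences take priority, stopping any single sequence and blocking new ones while active.
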(event EventBeginPlay)

(event EventTick
  (params (DeltaSeconds :type Float%20%28single-precision%29)))

(event EventShowHideBossHPBar
  (params (InShowing :type Boolean))
  (bind _localusahud (Variables|Default|GetLocalUSAHUD))
  ;[1 1 1] Comment
  (Utilities|IsValid _localusahud
    (:Is%20Valid
      (Class|USAHUD|ShowHideBossHPBar _localusahud InShowing))))

(event EventUpdateBossName
  (params (InName :type Name :default "None"))
  (bind _localusahud (Variables|Default|GetLocalUSAHUD))
  ;[1 1 1] Comment
  (Utilities|IsValid _localusahud
    (:Is%20Valid
      (Class|USAHUD|UpdateBossName _localusahud InName))))

(event EventPlayLevelSequenceMulti
  (params (InLevelSequence :type Level%20Sequence%20Actor%20Object%20Reference))
  (Utilities|IsValid (Variables|Default|GetLocalUSACharacter)
    (:Is%20Valid
      (Utilities|IsValid (Variables|Default|GetLocalUSAHUD)
        (:Is%20Valid
          ;[1 1 1] Comment
          (bind _output_get (Variables|Default|SetMultiLevelSeqeunceActor InLevelSequence))
          (Utilities|IsValid (Variables|Default|GetSingleLevelSeqeunceActor)
            (:Is%20Valid
              (Sequencer|Player|Stop (Variables|/Script/LevelSequence.LevelSequenceActor|GetSequencePlayer (Variables|Default|GetSingleLevelSeqeunceActor)) :!class /Script/MovieScene.MovieSceneSequencePlayer)
              (Variables|Default|SetSingleLevelSeqeunceActor 0))
            (:Is%20Not%20Valid
              _))
          ;[1 1 1] Comment
          (Class|USACharacterPlayer|SetLocalPlayerControllerInput (Variables|Default|GetLocalUSACharacter) false)
          (Class|USAHUD|PlayUserWidgetAnimationPanel (Variables|Default|GetLocalUSAHUD) false false)
          (Utilities|FlowControl|Delay 0.2)
          (Class|USAHUD|ShowHideCharacterHUD (Variables|Default|GetLocalUSAHUD) false)
          (Class|USAHUD|PlayUserWidgetAnimationPanel (Variables|Default|GetLocalUSAHUD) true false)
          ;[1 1 1] Comment
          (Class|USAGameStateBase|PlayLevelSequenceCore _output_get)
          (Utilities|FlowControl|Delay (- (Class|TimeManagementBlueprintLibrary|ToSeconds(QualifiedFrameTime) (Media|MediaPlayer|GetDuration (Variables|/Script/LevelSequence.LevelSequenceActor|GetSequencePlayer _output_get))) 0.2))
          ;[1 1 1] Comment
          (Class|USAHUD|PlayUserWidgetAnimationPanel (Variables|Default|GetLocalUSAHUD) false false)
          (Utilities|FlowControl|Delay 0.2)
          (Class|USAHUD|ShowHideCharacterHUD (Variables|Default|GetLocalUSAHUD) true)
          (Class|USAHUD|PlayUserWidgetAnimationPanel (Variables|Default|GetLocalUSAHUD) true false)
          (Class|USACharacterPlayer|SetLocalPlayerControllerInput (Variables|Default|GetLocalUSACharacter) true)
          (Variables|Default|SetMultiLevelSeqeunceActor 0))))))

(event EventUpdateBossHealthRatio
  (params (InRatio :type Float%20%28single-precision%29))
  (bind _localusahud (Variables|Default|GetLocalUSAHUD))
  ;[1 1 1] Comment
  (Utilities|IsValid _localusahud
    (:Is%20Valid
      (Class|USAHUD|UpdateBossHealthRatio _localusahud InRatio))))

(event EventPlayLevelSequenceSingle
  (params (InLevelSequence :type Level%20Sequence%20Actor%20Object%20Reference))
  (Utilities|IsValid (Variables|Default|GetLocalUSACharacter)
    (:Is%20Valid
      (Utilities|IsValid (Variables|Default|GetLocalUSAHUD)
        (:Is%20Valid
          ;[1 1 1] Comment
          (Utilities|IsValid (Variables|Default|GetMultiLevelSeqeunceActor)
            (:Is%20Not%20Valid
              (bind _output_get (Variables|Default|SetSingleLevelSeqeunceActor InLevelSequence))
              ;[1 1 1] Comment
              (Class|USACharacterPlayer|SetLocalPlayerControllerInput (Variables|Default|GetLocalUSACharacter) false)
              (Class|USAHUD|PlayUserWidgetAnimationPanel (Variables|Default|GetLocalUSAHUD) false false)
              (Utilities|FlowControl|Delay 0.2)
              (Class|USAHUD|ShowHideCharacterHUD (Variables|Default|GetLocalUSAHUD) false)
              (Class|USAHUD|PlayUserWidgetAnimationPanel (Variables|Default|GetLocalUSAHUD) true false)
              (Utilities|IsValid (Variables|Default|GetSingleLevelSeqeunceActor)
                (:Is%20Valid
                  ;[1 1 1] Comment
                  (Class|USAGameStateBase|PlayLevelSequenceCore _output_get)
                  (Utilities|FlowControl|Delay (- (Class|TimeManagementBlueprintLibrary|ToSeconds(QualifiedFrameTime) (Media|MediaPlayer|GetDuration (Variables|/Script/LevelSequence.LevelSequenceActor|GetSequencePlayer _output_get))) 0.2))
                  (Utilities|IsValid (Variables|Default|GetSingleLevelSeqeunceActor)
                    (:Is%20Valid
                      ;[1 1 1] Comment
                      (Class|USAHUD|PlayUserWidgetAnimationPanel (Variables|Default|GetLocalUSAHUD) false false)
                      (Utilities|FlowControl|Delay 0.2)
                      (Class|USAHUD|ShowHideCharacterHUD (Variables|Default|GetLocalUSAHUD) true)
                      (Class|USAHUD|PlayUserWidgetAnimationPanel (Variables|Default|GetLocalUSAHUD) true false)
                      (Class|USACharacterPlayer|SetLocalPlayerControllerInput (Variables|Default|GetLocalUSACharacter) true)
                      (Variables|Default|SetSingleLevelSeqeunceActor 0))))))))))))

(fn ConstructionScript)